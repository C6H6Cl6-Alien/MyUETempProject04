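; Player controller that shows an interaction prompt and lets the player interact with nearby actors.
; BeginPlay adds the main and button widgets to the viewport, the latter hidden, and caches all InteractiveActorBase actors once.
; Tick scans that list by distance to the pawn to track the nearest actor, toggling the button and IsInteractive by a fixed range.
; Pressing F calls Interact on that actor while IsInteractive is set.
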(event `self.ReceiveBeginPlay`
  (`|ExecutionSequence`
    (:`then_0`
      (bind _returnvalue (`|CreateWidget` "/Game/Blueprints/MainWidget.MainWidget_C"))
      (bind _output_get (set `self.MainWidget` _returnvalue))
      (`UserWidget.AddToViewport` _output_get 0))
    (:`then_1`
      (bind _returnvalue_2 (`|CreateWidget` "/Game/Blueprints/ButtonWidget.ButtonWidget_C"))
      (bind _output_get_2 (set `self.ButtonWidget` _returnvalue_2))
      (`UserWidget.AddToViewport` _output_get_2 0)
      (`Widget.SetVisibility` _output_get_2 "Hidden"))
    (:`then_2`
      (bind _outactors (`GameplayStatics.GetAllActorsOfClass` "/Game/Blueprints/InteractiveActorBase.InteractiveActorBase_C"))
      (set `self.InteractiveActors` _outactors))))

(event `self.ReceiveTick`
  (params (DeltaSeconds :type "Float (single-precision)"))
  (bind _interactiveactors (`self.InteractiveActors`))
  (bind _buttonwidget (`self.ButtonWidget`))
  (`|ExecutionSequence`
    (:`then_0`
      (set `self.PawnLocation` (`self.K2_GetActorLocation` (`GameplayStatics.GetPlayerPawn` 0)))
      (set `self.NearestInteractiveActorDistance` 2147483648.0))
    (:`then_1`
      (if (`KismetArrayLibrary.Array_IsNotEmpty` _interactiveactors)
        (for _array_element _interactiveactors
          (if (== (`self.NearestInteractiveActor`) null)
            (set `self.NearestInteractiveActor` _array_element)
            (else
              (bind _returnvalue (`KismetMathLibrary.Vector_Distance` (`self.K2_GetActorLocation` _array_element) (`self.PawnLocation`)))
              (if (< _returnvalue (`self.NearestInteractiveActorDistance`))
                (set `self.NearestInteractiveActor` _array_element)
                (set `self.NearestInteractiveActorDistance` _returnvalue)))))
        (else
          (set `self.NearestInteractiveActor` null)
          (set `self.NearestInteractiveActorDistance` 2147483648.0))))
    (:`then_2`
      (if (and (!= (`self.NearestInteractiveActor`) null) (<= (`self.NearestInteractiveActorDistance`) 400.0))
        (`Widget.SetVisibility` _buttonwidget "Visible")
        (set `self.IsInteractive` true)
        (else
          (`Widget.SetVisibility` _buttonwidget "Hidden")
          (set `self.IsInteractive` false))))))

(event `Key|F`
  (params (Key :type "Key Structure"))
  (:`Pressed`
    (if (`self.IsInteractive`)
      (`/Game/Blueprints/InteractiveActorBase.Interact` (`self.NearestInteractiveActor`)))))

(fn `UserConstructionScript`)