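; Interactive door actor that opens and closes when its Interact function is called.
; Interact toggles IsOpen, swaps the InteractiveText prompt between Open and Close, and instantly rotates DoorMesh a quarter turn around yaw with a local rotation, without animation.
; The construction script sets the initial prompt to Open, and the event graph holds only disabled default events.
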(fn `Interact`
  (bind _doormesh (`self.DoorMesh`))
  (if (`self.IsOpen`)
    (set `self.IsOpen` false)
    (set `self.InteractiveText` "Open")
    (`SceneComponent.K2_AddLocalRotation` _doormesh (struct :`Yaw` -90.0) false false)
    (else
      (set `self.IsOpen` true)
      (set `self.InteractiveText` "Close")
      (`SceneComponent.K2_AddLocalRotation` _doormesh (struct :`Yaw` 90.0) false false))))

(fn `UserConstructionScript`
  (`parent.UserConstructionScript`)
  (set `self.InteractiveText` "Open"))