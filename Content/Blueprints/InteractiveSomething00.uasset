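; InteractiveSomething00 is an interactive actor that broadcasts a random color to other interactive objects when used.
; On BeginPlay it caches every InteractiveSomethingBase actor in the level.
; Its Interact override runs the parent logic, then builds a random RGB vector and passes it to SomeFunc on each cached actor.
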(event `self.ReceiveBeginPlay`
  (`parent.ReceiveBeginPlay`)
  (bind _outactors (`GameplayStatics.GetAllActorsOfClass` "/Game/Blueprints/InteractiveSomethingBase.InteractiveSomethingBase_C"))
  (set `self.Something` _outactors))

(fn `Interact`
  (locals (Color :type "Vector Structure" :default (0.0 0.0 0.0)))
  (`parent.Interact`)
  (bind _output_get (set `local.Color` (`KismetMathLibrary.MakeVector` (`KismetMathLibrary.RandomFloatInRange` 0.0 1.0) (`KismetMathLibrary.RandomFloatInRange` 0.0 1.0) (`KismetMathLibrary.RandomFloatInRange` 0.0 1.0))))
  (for _array_element (`self.Something`)
    (`self.SomeFunc` _array_element _output_get)))

(fn `UserConstructionScript`
  (`parent.UserConstructionScript`))