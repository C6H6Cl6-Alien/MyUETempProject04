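; MyGameState runs a day/night cycle, keeping a 24-hour clock and rotating the level's directional light to match.
; BeginPlay starts the clock at 6:00 and caches the DirectionalLight found in the level.
; While that light reference is set, Tick advances CurrentHour by real minutes scaled by TimeFlowMultiplier, wrapping at 24.
; The hour maps linearly to sun pitch at 15 degrees per hour, with fixed yaw.
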(event `self.ReceiveBeginPlay`
  (`|ExecutionSequence`
    (:`then_0`
      (set `self.CurrentHour` 6.0))
    (:`then_1`
      (bind _returnvalue (`GameplayStatics.GetActorOfClass` "/Script/Engine.DirectionalLight"))
      (set `self.DirectionalLight` _returnvalue))))

(event `self.ReceiveTick`
  (params (DeltaSeconds :type "Float (single-precision)"))
  (if (not (== (`self.DirectionalLight`) null))
    (bind _output_get (set `self.CurrentHour` (+ (* (/ DeltaSeconds 60.0) (`self.TimeFlowMultiplier`)) (`self.CurrentHour`))))
    (if (>= _output_get 24.0)
      (set `self.CurrentHour` (- _output_get 24.0)))
    (`self.K2_SetActorRotation` (`self.DirectionalLight`) (`KismetMathLibrary.MakeRotator` 0.0 (* (- 30.0 _output_get) 15.0) 270.0) false)))

(fn `UserConstructionScript`)