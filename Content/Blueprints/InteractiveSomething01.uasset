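; Interactable Blueprint that cycles the game's time flow speed each time it is used.
; BeginPlay caches the game state as MyGameState, and the Interact override writes directly to its TimeFlowMultiplier.
; A chain of equality checks steps the multiplier through normal, double, quadruple and half speed, resetting to normal from half or any unexpected value.
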(event `self.ReceiveBeginPlay`
  (`parent.ReceiveBeginPlay`)
  (bind _asmy_game_state (cast `/Game/Blueprints/MyGameState` (`GameplayStatics.GetGameState`)))
  (set `self.GameState` _asmy_game_state))

(fn `Interact`
  (`parent.Interact`)
  (if (== (`/Game/Blueprints/MyGameState.TimeFlowMultiplier` (`self.GameState`)) 1.0)
    (set `/Game/Blueprints/MyGameState.TimeFlowMultiplier` 2.0 (`self.GameState`))
    (elif (== (`/Game/Blueprints/MyGameState.TimeFlowMultiplier` (`self.GameState`)) 2.0)
      (set `/Game/Blueprints/MyGameState.TimeFlowMultiplier` 4.0 (`self.GameState`))
      (elif (== (`/Game/Blueprints/MyGameState.TimeFlowMultiplier` (`self.GameState`)) 4.0)
        (set `/Game/Blueprints/MyGameState.TimeFlowMultiplier` 0.5 (`self.GameState`))
        (else
          (if (== (`/Game/Blueprints/MyGameState.TimeFlowMultiplier` (`self.GameState`)) 0.5)
            _
            (else
              _))
          (set `/Game/Blueprints/MyGameState.TimeFlowMultiplier` 1.0 (`self.GameState`)))))))

(fn `UserConstructionScript`
  (`parent.UserConstructionScript`))