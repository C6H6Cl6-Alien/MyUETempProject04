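; Interactive actor that works as a light switch for every Bulb actor in the level.
; It caches all Bulb actors at BeginPlay, then on Interact calls the parent and flips each bulb's PointLight intensity between off and a fixed brightness.
; Each bulb toggles on its own current state, so InteractiveText ("Turn on" or "Turn off") reflects the last bulb processed.
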(event `self.ReceiveBeginPlay`
  (`parent.ReceiveBeginPlay`)
  (bind _outactors (`GameplayStatics.GetAllActorsOfClass` "/Game/Blueprints/Bulb.Bulb_C"))
  (set `self.Bulbs` _outactors))

(fn `Interact`
  (`parent.Interact`)
  (for _array_element (`self.Bulbs`)
    (bind _pointlight (`/Game/Blueprints/Bulb.PointLight` _array_element))
    (if (== (`LightComponentBase.Intensity` _pointlight) 0.0)
      (`LightComponent.SetIntensity` _pointlight 1000.0)
      (set `self.InteractiveText` "Turn off")
      (else
        (`LightComponent.SetIntensity` _pointlight 0.0)
        (set `self.InteractiveText` "Turn on")))))

(fn `UserConstructionScript`
  (`parent.UserConstructionScript`))