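; An interactive actor that toggles the light color temperature of every Bulb actor in the level.
; On BeginPlay it caches all Bulb actors through GetAllActorsOfClass.
; Its Interact override calls the parent, then flips each bulb's PointLight between a cool and a warm temperature.
; The interaction text updates inside the same loop to name the opposite color, so the last bulb processed decides the prompt.
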(event `self.ReceiveBeginPlay`
  (`parent.ReceiveBeginPlay`)
  (bind _outactors (`GameplayStatics.GetAllActorsOfClass` "/Game/Blueprints/Bulb.Bulb_C"))
  (set `self.Bulbs` _outactors))

(fn `Interact`
  (`parent.Interact`)
  (for _array_element (`self.Bulbs`)
    (bind _pointlight (`/Game/Blueprints/Bulb.PointLight` _array_element))
    (if (== (`LightComponent.Temperature` _pointlight) 6500.0)
      (`LightComponent.SetTemperature` _pointlight 5000.0)
      (set `self.InteractiveText` "Set cool color")
      (else
        (`LightComponent.SetTemperature` _pointlight 6500.0)
        (set `self.InteractiveText` "Set warm color")))))

(fn `UserConstructionScript`
  (`parent.UserConstructionScript`))